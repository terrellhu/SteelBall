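; Player pawn moved by physics torque, with a camera fade-in on start and a level restart on failure.
; Both movement axes feed one AddTorque call as an amplified acceleration change, gated by CanMove.
; BeginPlay enables movement and creates the BP_UI widget, while any damage fades the camera out before reloading the level.
; AdjustCamera sets the spring arm's length and world rotation.
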(event EventBeginPlay
  ;[1 1 1] 开局淡入
  (Variables|Default|SetCanMove true)
  (Utilities|CameraFade :FromAlpha 1.0 :Duration (Math|Float|MakeLiteralFloat 1.0))
  ;[1 1 1] 创建UI
  (bind _returnvalue (UserInterface|CreateWidget "/Game/Blueprints/BP_UI.BP_UI_C"))
  (UserInterface|Viewport|AddtoViewport _returnvalue 0))

(event Game|Damage|EventAnyDamage
  (params (Damage :type Float%20%28single-precision%29) (DamageType :type Damage%20Type%20Object%20Reference) (InstigatedBy :type Controller%20Object%20Reference) (DamageCauser :type Actor%20Object%20Reference))
  (bind _returnvalue (Math|Float|MakeLiteralFloat 1.0))
  ;[1 1 1] 失败淡出
  (Utilities|CameraFade :ToAlpha 1.0 :Duration _returnvalue :bHoldWhenFinished true)
  (Utilities|FlowControl|Delay _returnvalue)
  (Utilities|RestartLevel))

(event Input|AxisEvents|InputAxisMoveF/B
  (params (AxisValue :type Float%20%28single-precision%29))
  (bind _amplificaction (Variables|PlayerMove|GetAmplificaction))
  ;[1 1 1] PlayerMove
  (if (Variables|Default|GetCanMove)
    (Class|PrimitiveComponent|AddTorqueinRadians (Variables|Default|GetPlayer) (Math|Vector|MakeVector (* (stale Input|AxisEvents|InputAxisMoveL/R AxisValue) _amplificaction) (* AxisValue _amplificaction) 0.0) "None" true)))

(event Input|AxisEvents|InputAxisMoveL/R
  (params (AxisValue :type Float%20%28single-precision%29))
  (bind _amplificaction (Variables|PlayerMove|GetAmplificaction))
  ;[1 1 1] PlayerMove
  (if (Variables|Default|GetCanMove)
    (Class|PrimitiveComponent|AddTorqueinRadians (Variables|Default|GetPlayer) (Math|Vector|MakeVector (* AxisValue _amplificaction) (* (stale Input|AxisEvents|InputAxisMoveF/B AxisValue) _amplificaction) 0.0) "None" true)))

(fn ConstructionScript)

(fn AdjustCamera
  (params (ArmLength :type Float%20%28single-precision%29) (Rotation :type Rotator))
  (bind _springarm (Variables|Default|GetSpringArm))
  (Variables|/Script/Engine.SpringArmComponent|SetTargetArmLength _springarm ArmLength)
  (Transformation|SetWorldRotation _springarm Rotation false false))