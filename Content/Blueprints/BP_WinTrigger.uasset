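; Level exit trigger that lets the player finish a level once every crystal is collected.
; On BeginPlay it stores the level's BP_Crystal count in the GameInstance and resets the collected count.
; On player overlap with all crystals, it saves BP_UI's level time, then opens the next LevelNames entry or, on the last, sets IsWin and disables player movement.
; If crystals are missing, it plays the BP_UI blink animation instead.
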(event Collision|EventActorBeginOverlap
  (params (OtherActor :type Actor%20Object%20Reference))
  ;[1 1 1] 判断是否收集完所有水晶，成功则存储关卡时间
  (Utilities|IsPlayer OtherActor
    (:True
      (if (CallFunction|IsAllCrystalCollected)
        (CallFunction|SaveLevelTime)
        (if (CallFunction|IsLastLevel)
          (Variables|/Game/Blueprints/BP_GameInstance.BP_GameInstance_C|SetIsWin (Utilities|GetGameInstance) true)
          (Variables|/Game/Blueprints/BP_Player.BP_Player_C|SetCanMove (.AsBP%20Player (Utilities|Casting|CastToBP_Player (Game|Player|GetPlayerPawn 0))) false)
          (else
            (CallFunction|LoadNextLevel)))
        (else
          (bind _foundwidgets (Widget|GetAllWidgetsOfClass "/Game/Blueprints/BP_UI.BP_UI_C" true))
          (Default|PlayBlinkAnimation (Utilities|Array|Get(acopy) _foundwidgets)))))))

(event EventBeginPlay
  (bind _gameinstance (Utilities|GetGameInstance))
  ;[1 1 1] 取得关卡中水晶总数
  (bind _outactors (Actor|GetAllActorsOfClass "/Game/Blueprints/BP_Crystal.BP_Crystal_C"))
  (Variables|/Game/Blueprints/BP_GameInstance.BP_GameInstance_C|SetAllCrystalNum _gameinstance (Utilities|Array|Length _outactors))
  (Variables|/Game/Blueprints/BP_GameInstance.BP_GameInstance_C|SetCollectedCrystalNum _gameinstance 0))

(fn ConstructionScript)

(fn SaveLevelTime
  (bind _foundwidgets (Widget|GetAllWidgetsOfClass "/Game/Blueprints/BP_UI.BP_UI_C" true))
  (Variables|/Game/Blueprints/BP_GameInstance.BP_GameInstance_C|SetGameTime (Utilities|GetGameInstance) (Variables|/Game/Blueprints/BP_UI.BP_UI_C|GetLevelTime (Utilities|Array|Get(acopy) _foundwidgets))))

(fn IsAllCrystalCollected
  (bind _gameinstance (Utilities|GetGameInstance))
  (return (== (Variables|/Game/Blueprints/BP_GameInstance.BP_GameInstance_C|GetAllCrystalNum _gameinstance) (Variables|/Game/Blueprints/BP_GameInstance.BP_GameInstance_C|GetCollectedCrystalNum _gameinstance))))

(fn IsLastLevel
  (return (== (Utilities|Array|LastIndex (Variables|Default|GetLevelNames)) (CallFunction|GetLevelIndex))))

(fn GetLevelIndex
  (bind _returnvalue (Game|GetCurrentLevelName true))
  (return (Utilities|Array|FindItem (Variables|Default|GetLevelNames) (Utilities|String|StringToName _returnvalue))))

(fn LoadNextLevel
  (bind _result (Math|Integer|IncrementInt (CallFunction|GetLevelIndex))
    (:%20%20
      (Game|OpenLevel(byName) (Utilities|Array|Get(acopy) (Variables|Default|GetLevelNames) _result)))))