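; BP_Cannon is an automatic cannon that repeatedly fires BP_Projectile actors from the moment play begins.
; Each cycle waits FireRate, activates the fire particle, spawns a scaled projectile at ProjectileSpawnPoint and restarts CannonFireTimeline.
; The timeline animates the Cannon component's relative location, and its Fire Event track loops back to the delay, so the timeline itself drives the repeat.
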(event EventBeginPlay
  (Utilities|FlowControl|Delay (Variables|CannonSetting|GetFireRate) :!label _label)
  (Components|Activation|Activate (Variables|Default|GetFireParticle) true)
  (CallFunction|SpawnProjectile)
  (bind _firelocation (Timeline|CannonFireTimeline PlayFromStart)
    (:Update
      (CallFunction|FireAnimation _firelocation))
    (:FireEvent
      (goto _label))))

(fn ConstructionScript)

(fn SpawnProjectile
  (bind _projectilespawnpoint (Variables|Default|GetProjectileSpawnPoint))
  (Game|SpawnActorfromClass "/Game/Blueprints/BP_Projectile.BP_Projectile_C" (Math|Transform|MakeTransform (Transformation|GetWorldLocation _projectilespawnpoint) (Transformation|GetWorldRotation _projectilespawnpoint) (Math|Conversions|ToVector(Float) (Variables|CannonSetting|GetProjectileScale))) "Undefined" 0 0))

(fn FireAnimation
  (params (NewLocation_Y :type Float%20%28single-precision%29))
  (Transformation|SetRelativeLocation (Variables|Default|GetCannon) (Math|Vector|MakeVector 0.0 NewLocation_Y 0.0) false false))