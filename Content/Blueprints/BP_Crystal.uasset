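; BP_Crystal is a collectible crystal that the player picks up by overlapping it.
; An IsPlayer check filters overlaps, then the current location, scale and light intensity are saved as lerp start values.
; CollectTimeline's three alpha tracks pull the crystal toward the player's live position while shrinking it and fading its PointLight.
; When the timeline finishes, the actor destroys itself and calls OnCrystalCollect on the GameInstance.
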(event Collision|EventActorBeginOverlap
  (params (OtherActor :type Actor%20Object%20Reference))
  (Utilities|IsPlayer OtherActor
    (:True
      (CallFunction|SaveStartValue)
      (bind (_direction _locationalpha _scalealpha _intensityalpha) (Timeline|CollectTimeline Play)
        (:Update
          (CallFunction|CollectLocation _locationalpha)
          (CallFunction|CollectScale _scalealpha)
          (CallFunction|CollectIntensity _intensityalpha))
        (:Finished
          (Actor|DestroyActor)
          (Default|OnCrystalCollect (Utilities|GetGameInstance)))))))

(fn ConstructionScript)

(fn SaveStartValue
  (Variables|SaveValue|SetStartLocation (Transformation|GetActorLocation))
  (Variables|SaveValue|SetStartScale (Transformation|GetActorScale3D))
  (Variables|SaveValue|SetStartIntensity (Variables|/Script/Engine.LightComponentBase|GetIntensity (Variables|Default|GetPointLight))))

(fn CollectLocation
  (params (Alpha :type Float%20%28single-precision%29))
  (Transformation|SetActorLocation (Math|Vector|Lerp(Vector) (Variables|SaveValue|GetStartLocation) (Transformation|GetActorLocation (Game|Player|GetPlayerPawn 0)) Alpha) false false))

(fn CollectScale
  (params (Alpha :type Float%20%28single-precision%29))
  (Transformation|SetActorScale3D (Math|Vector|Lerp(Vector) (Variables|SaveValue|GetStartScale) "0, 0, 0" Alpha)))

(fn CollectIntensity
  (params (Alpha :type Float%20%28single-precision%29))
  (Rendering|Components|Light|SetIntensity (Variables|Default|GetPointLight) (Math|Float|Lerp (Variables|SaveValue|GetStartIntensity) 0.0 Alpha)))