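; Spotlight actor that turns its SpotLight to follow the player once the player overlaps it.
; Begin and end overlap events filter for the player, and both set the tracking flag true, so tracking continues after the player leaves.
; While the flag is set, Tick smoothly interpolates the light's world rotation toward a look-at rotation on the first player's pawn.
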(event Collision|EventActorBeginOverlap
  (params (OtherActor :type Actor%20Object%20Reference))
  ;[1 1 1] 检测玩家是否在触发区域中
  (Utilities|IsPlayer OtherActor
    (:True
      (Variables|Default|SetIsPlayerOverlaping true))))

(event EventTick
  (params (DeltaSeconds :type Float%20%28single-precision%29))
  (bind _spotlight (Variables|Default|GetSpotLight))
  ;[1 1 1] 通过插值使聚光灯跟随玩家
  (if (Variables|Default|GetIsPlayerOverlaping)
    (Transformation|SetWorldRotation _spotlight (Math|Interpolation|RInterpTo (Transformation|GetWorldRotation _spotlight) (Math|Rotator|FindLookatRotation (Transformation|GetWorldLocation _spotlight) (Transformation|GetActorLocation (Game|Player|GetPlayerPawn 0))) DeltaSeconds 2.0) false false)))

(event Collision|EventActorEndOverlap
  (params (OtherActor :type Actor%20Object%20Reference))
  ;[1 1 1] 检测玩家是否在触发区域中
  (Utilities|IsPlayer OtherActor
    (:True
      (Variables|Default|SetIsPlayerOverlaping true))))

(fn ConstructionScript)